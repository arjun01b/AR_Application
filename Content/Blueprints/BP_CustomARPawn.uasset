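; Player pawn that runs the game's menu flow and countdown timer.
; BeginPlay shows a paused main menu after a short delay and binds its buttons to open how-to-play or settings widgets, or start play with a Timer widget.
; While GameState is true, Tick uses a one-second Delay to throttle the Minutes/Seconds countdown, showing GameOver and pausing at zero.
; PlayGame sets SoundToggle but never GameState.
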(event Custom|SettingsButtonClick
  (bind _returnvalue (UserInterface|CreateWidget "/Game/Widgets/SettingsWidget.SettingsWidget_C"))
  (UserInterface|Viewport|AddtoViewport _returnvalue 0))

(event Custom|HowToPlayButtonClicked
  (bind _returnvalue (UserInterface|CreateWidget "/Game/Widgets/NewWidgetBlueprint.NewWidgetBlueprint_C"))
  (UserInterface|Viewport|AddtoViewport _returnvalue 0))

(event Custom|PlayGame
  (bind _returnvalue (Game|GetPlayerController 0))
  (Variables|Default|SetSoundToggle true)
  (Viewport|RemoveAllWidgets)
  (bind _returnvalue_2 (UserInterface|CreateWidget "/Game/Widgets/Timer.Timer_C"))
  (UserInterface|Viewport|AddtoViewport _returnvalue_2 0)
  (Input|SetInputModeGameOnly _returnvalue)
  (Variables|/Script/Engine.PlayerController|SetbShowMouseCursor _returnvalue true)
  (Game|SetGamePaused false))

(event EventTick
  (params (DeltaSeconds :type Float%20%28single-precision%29))
  (Utilities|FlowControl|Sequence
    (:then_0
      (if (Variables|Default|GetgameState)
        (Utilities|FlowControl|Delay 1.0)
        (if (== (Variables|Default|GetSeconds) 0)
          (if (== (Variables|Default|GetMinutes) 0)
            (bind _returnvalue (UserInterface|CreateWidget "/Game/Widgets/GameOver.GameOver_C"))
            (UserInterface|Viewport|AddtoViewport _returnvalue 0)
            (Variables|/Script/Engine.PlayerController|SetbShowMouseCursor (Game|GetPlayerController 0) true)
            (Game|SetGamePaused true)
            (else
              (Variables|Default|SetSeconds 59)
              (Variables|Default|SetMinutes (- (Variables|Default|GetMinutes) 1))))
          (else
            (Variables|Default|SetSeconds (- (Variables|Default|GetSeconds) 1))))))))

(event Collision|EventActorBeginOverlap
  (params (OtherActor :type Actor%20Object%20Reference)))

(event EventBeginPlay
  (bind _returnvalue (Game|GetPlayerController 0))
  (Utilities|FlowControl|Sequence
    (:then_0
      (Utilities|FlowControl|Delay 0.2)
      (bind _returnvalue_2 (UserInterface|CreateWidget "/Game/Widgets/MainMenu_widget.MainMenu_widget_C"))
      (bind _output_get (Variables|Default|SetMainMenu_Ref _returnvalue_2))
      (UserInterface|Viewport|AddtoViewport _output_get 0)
      (Game|SetGamePaused true)
      (Input|SetInputModeUIOnly _returnvalue (Variables|Default|GetMainMenu_Ref) "DoNotLock")
      (Variables|/Script/Engine.PlayerController|SetbShowMouseCursor _returnvalue true)
      (EventDispatchers|AssignOnClicked (Variables|/Game/Widgets/MainMenu_widget.MainMenu_widget_C|GetHowToPlayButton (Variables|Default|GetMainMenu_Ref)) (delegate Custom|HowToPlayButtonClicked))
      (EventDispatchers|AssignOnClicked (Variables|/Game/Widgets/MainMenu_widget.MainMenu_widget_C|GetSettingsButton (Variables|Default|GetMainMenu_Ref)) (delegate Custom|SettingsButtonClick))
      (EventDispatchers|AssignOnClicked (Variables|/Game/Widgets/MainMenu_widget.MainMenu_widget_C|GetPlayButton (Variables|Default|GetMainMenu_Ref)) (delegate Custom|PlayGame)))))

(fn ConstructionScript)